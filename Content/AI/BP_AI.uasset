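; Zombie enemy character that takes damage, attacks in melee and adds to the player's kill count when it dies.
; At zero health it ragdolls, stops moving, increments the first-person character's dead counter and is destroyed after a short delay.
; AttackAI plays an attack montage while alive, using its notify to time a short forward sphere trace that damages the pawn it hits.
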(event EventAttackAI
  (bind _returnvalue (Transformation|GetActorLocation))
  (if (not (Variables|Default|GetisDead))
    (Animation|Montage|PlayMontage (Variables|Character|GetMesh) "/Game/Characters/Enemy/Zombie_Attack_Anim_Montage.Zombie_Attack_Anim_Montage"
      (:OnNotifyBegin
        (bind (_outhit _returnvalue_2) (Collision|SphereTraceForObjects _returnvalue (+ _returnvalue (* (Math|Vector|GetForwardVector (Transformation|GetActorRotation)) 1e+02)) 3e+01 (Utilities|Array|MakeArray "ObjectTypeQuery3") false 0 "None"))
        (if _returnvalue_2
          (Game|Damage|ApplyDamage (.HitActor (Collision|BreakHitResult _outhit)) 2e+01 0 0))))))

(event Game|Damage|EventAnyDamage
  (params (Damage :type Float%20%28single-precision%29) (DamageType :type Damage%20Type%20Object%20Reference) (InstigatedBy :type Controller%20Object%20Reference) (DamageCauser :type Actor%20Object%20Reference))
  (Variables|Default|Sethealth (- (Variables|Default|Gethealth) Damage))
  (if (<= (Variables|Default|Gethealth) 0.0)
    (Physics|SetSimulatePhysics (Variables|Character|GetMesh) true)
    (Variables|Default|SetisDead true)
    (Pawn|Components|CharacterMovement|DisableMovement (Variables|Character|GetCharacterMovement))
    (Utilities|FlowControl|Sequence
      (:then_0
        (bind _asbp_first_person_character_1 (Utilities|Casting|CastToBP_FirstPersonCharacter1 (Game|GetPlayerCharacter 0)))
        (Math|Integer|IncrementInt (Variables|/Game/FirstPerson/Blueprints/BP_FirstPersonCharacter1.BP_FirstPersonCharacter1_C|GetAddDead _asbp_first_person_character_1)
          (:%20%20
            (Collision|SetCollisionEnabled (Variables|Character|GetMesh) "PhysicsOnly"))))
      (:then_1
        (Utilities|FlowControl|Delay 2.0)
        (Actor|DestroyActor)))))

(fn ConstructionScript)