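; A weapon pickup actor that gives the interacting character a weapon.
; On Interact, it calls SpawnWeapon on the passed CharacterPickUps with its WeaponToSpawn value, then destroys itself.
; A debug "spawn" string prints on interaction, and the default BeginPlay, overlap and Tick events are unused.
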(event EventBeginPlay
  (|CallParentFunction) ; This node is disabled and will not be called.\nDrag off pins to build functionality.
)

(event Collision|EventActorBeginOverlap
  (params (OtherActor :type Actor%20Object%20Reference))
  (|CallParentFunction OtherActor) ; This node is disabled and will not be called.\nDrag off pins to build functionality.
)

(event EventTick
  (params (DeltaSeconds :type Float%20%28single-precision%29))
  (|CallParentFunction DeltaSeconds) ; This node is disabled and will not be called.\nDrag off pins to build functionality.
)

(event EventInteract
  (params (CharacterPickUps :type BP%20First%20Person%20Character%201%20Object%20Reference))
  (Development|PrintString "spawn")
  (Default|SpawnWeapon CharacterPickUps (Variables|Default|GetWeaponToSpawn))
  (Actor|DestroyActor))

(fn ConstructionScript
  (|CallParentFunction))